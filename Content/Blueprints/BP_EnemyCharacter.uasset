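; BP_EnemyCharacter is an enemy character that displays its current health as colored text.
; It sets the text from HealthComponent on BeginPlay, starting in the healthy color, then updates value and color on each OnHealthChanged event.
; GetColorFromHealthValue picks healthy, hurt or critical color using fixed health thresholds.
; OnDeath only hides the health text; Tick and overlap events are empty.
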(event `self.ReceiveBeginPlay`
  (bind _healthtext (`self.HealthText`))
  (`TextRenderComponent.K2_SetText` _healthtext (`KismetTextLibrary.Conv_DoubleToText` (`STS_HealthComponent.CurrentHealth` (`self.HealthComponent`)) "HalfToEven"))
  (`TextRenderComponent.SetTextRenderColor` _healthtext (`self.HealthyColor`)))

(event `self.HealthComponent.OnHealthChanged`
  (params (HealthComponent :type "STS_HealthComponent Object Reference") (Health :type "Float (single-precision)") (HealthDelta :type "Float (single-precision)") (DamageType :type "DamageType Object Reference") (InstigatedBy :type "Controller Object Reference") (DamageCauser :type "Actor Object Reference"))
  (bind _healthtext (`self.HealthText`))
  (`TextRenderComponent.K2_SetText` _healthtext (`KismetTextLibrary.Conv_DoubleToText` Health "HalfToEven"))
  (`TextRenderComponent.SetTextRenderColor` _healthtext (`self.GetColorFromHealthValue` Health)))

(event `self.HealthComponent.OnDeath`
  (params (HealthComponent :type "STS_HealthComponent Object Reference") (InstigatedBy :type "Controller Object Reference") (Killer :type "Actor Object Reference"))
  (`SceneComponent.SetVisibility` (`self.HealthText`) false false))

(fn `GetColorFromHealthValue`
  (params (CurrentHealth :type "Float (double-precision)"))
  (returns (HealthColor :type "Color Structure"))
  (return (select `bool` (> CurrentHealth 80.0) :`false` (select `bool` (> CurrentHealth 30.0) :`false` (`self.CriticalColor`) :`true` (`self.HurtColor`)) :`true` (`self.HealthyColor`))))

(fn `UserConstructionScript`)